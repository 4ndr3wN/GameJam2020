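; CustomPlayerController is a player controller marked obsolete, with empty BeginPlay and Tick events.
; Its disconnected logic would switch control to the first other PlayerCharacter whose IsPossesed flag is false, using UnPossess and Possess.
; A second unwired fragment prints a character's controller ID, and a TODO questions whether the switching belongs in the level blueprint.
; None of this logic runs.
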(event `self.ReceiveTick`
  (params (DeltaSeconds :type "Float (single-precision)"))
  ;[1 1 1] OBSOLETE
)

(fn `UserConstructionScript`)