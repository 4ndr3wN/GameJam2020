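; Player controller Blueprint that lets the player switch control between robot characters.
; On the SwitchRobot input, it scans all PlayerCharacter actors for one that is neither the current pawn nor flagged as possessed.
; It then unpossesses the current pawn and possesses the first match.
; Other events are empty, and a leftover debug print of controller IDs is unconnected.
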(event `InputAction|SwitchRobot`
  (params (Key :type "Key Structure"))
  (:`Pressed`
    (bind _outactors (`GameplayStatics.GetAllActorsOfClass` "/Game/Blueprints/PlayerCharacter.PlayerCharacter_C")) ; TODO: place in level blueprint?
    (for _array_element _outactors
      (if (!= _array_element (`self.K2_GetPawn` self))
        (if (not (`/Game/Blueprints/PlayerCharacter.IsPossesed` _array_element))
          (`self.UnPossess`)
          (`self.Possess` _array_element)
          (break))))))

(fn `UserConstructionScript`)