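; PlayerCharacter is a controllable character that lets its controller jump to another overlapping PlayerCharacter.
; Movement input drives it forward and yaws it, while overlap events track whether a swap is possible.
; The Pair action possesses the other character if it is unpossessed and this one's possession timer, counted on Tick, has reached its maximum.
; On becoming view target, it hands the view to the shared MainCamera-tagged camera.
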(event `InputAxis|MoveRight`
  (params (AxisValue :type "Float (single-precision)"))
  ;[1 1 1] Move Right
  (`self.AddControllerYawInput` AxisValue))

(event `InputAxis|MoveForward`
  (params (AxisValue :type "Float (single-precision)"))
  ;[1 1 1] Move Forward
  (`self.AddMovementInput` (`self.GetActorForwardVector`) AxisValue))

(event `InputAction|Pair`
  (params (Key :type "Key Structure"))
  (bind _returnvalue (`self.GetController`))
  ;[1 1 1] Possess
  (:`Pressed`
    (if (`self.canPress`)
      (if (not (`/Game/Blueprints/PlayerCharacter.IsPossesed` (stale `self.ReceiveActorBeginOverlap` _asplayer_character)))
        (if (<= (- (`self.PossesableMaxTime`) (`self.PossesionCurrentTimer`)) 0.0)
          (`/Engine/EditorBlueprintResources/StandardMacros.IsValid` _returnvalue
            (:`Is Valid`
              (`Controller.Possess` _returnvalue (stale `self.ReceiveActorBeginOverlap` _asplayer_character)))))))))

(event `self.ReceiveActorBeginOverlap`
  (params (OtherActor :type "Actor Object Reference"))
  ;[1 1 1] Collision check
  (bind _asplayer_character (cast `/Game/Blueprints/PlayerCharacter` OtherActor))
  (set `self.canPress` true)
  (`KismetSystemLibrary.PrintString` (`KismetStringLibrary.Conv_IntToString` (`GameplayStatics.GetPlayerControllerID` null))))

(event `self.ReceiveActorEndOverlap`
  (params (OtherActor :type "Actor Object Reference"))
  ;[1 1 1] Collision check
  (cast `/Game/Blueprints/PlayerCharacter` OtherActor)
  (set `self.canPress` false))

(event `self.ReceivePossessed`
  (params (NewController :type "Controller Object Reference"))
  ;[1 1 1] Possessed
  (set `self.IsPossesed` true)
  (set `self.PossesionCurrentTimer` 0.0))

(event `self.ReceiveUnpossessed`
  (params (OldController :type "Controller Object Reference"))
  ;[1 1 1] Unpossessed
  (set `self.IsPossesed` false))

(event `self.ReceiveBeginPlay`
  ;[1 1 1] Set Camera Reference
  (bind _outactors (`GameplayStatics.GetAllActorsOfClassWithTag` "/Script/Engine.CameraActor" "MainCamera"))
  (bind _ascamera_actor (cast `CameraActor` (`|GetArrayItem` _outactors)))
  (set `self.CameraReference` _ascamera_actor))

(event `self.ReceiveTick`
  (params (DeltaSeconds :type "Float (single-precision)"))
  ;[1 1 1] Possesion Timer
  (if (`self.IsPossesed`)
    (set `self.PossesionCurrentTimer` (+ DeltaSeconds (`self.PossesionCurrentTimer`)))))

(event `self.K2_OnBecomeViewTarget`
  (params (PC :type "PlayerController Object Reference"))
  ;[1 1 1] Set View Target
  (`PlayerController.SetViewTargetWithBlend` PC (`self.CameraReference`) 0.0 "VTBlend_Linear" 0.0 false))

(fn `UserConstructionScript`)