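; Freeze perk Blueprint that, when triggered, freezes every player character except the one who activates it.
; Its Effect override calls the parent effect, then loops over all PlayerCharacter actors in the world and calls Freeze on each one other than the passed-in player.
; The event graph holds only disabled default events, so all behavior lives in Effect.
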(fn `Effect`
  (params (PlayerChar :type "/Game/Blueprints/PlayerCharacter Object Reference"))
  (`parent.Effect` PlayerChar)
  (bind _outactors (`GameplayStatics.GetAllActorsOfClass` "/Game/Blueprints/PlayerCharacter.PlayerCharacter_C"))
  (for _array_element _outactors
    (if (not (== PlayerChar _array_element))
      (`/Game/Blueprints/PlayerCharacter.Freeze` _array_element))))

(fn `UserConstructionScript`
  (`parent.UserConstructionScript`))