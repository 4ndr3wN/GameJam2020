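; Player home base that holds an ordered list of random collectables to deliver and decides the match winner.
; On BeginPlay it builds the list from GameMode's count and GameInstance picks, spawning a row of preview meshes.
; Its DropArea flags the owning player; TryObjectDrop accepts only the first listed ID, removing that entry and mesh.
; Emptying the list freezes all players, with confetti on the winner and lightning on the loser.
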(event `self.ReceiveBeginPlay`
  ;[1 1 1] Getting the ingredients number for this match from game mode
  (bind _asin_game_mode (cast `/Game/Levels/InGameMode` (`GameplayStatics.GetGameMode`)))
  (bind _newparam (`/Game/Levels/InGameMode.GetCollectables` _asin_game_mode))
  (set `self.ListLength` _newparam)
  (bind _ascustom_game_instance (cast `/Game/CustomGameInstance` (`GameplayStatics.GetGameInstance`)))
  (for _ (range (`self.ListLength`))
    (bind _colectable (`/Game/CustomGameInstance.GetRandomCollectable` _ascustom_game_instance))
    (bind _returnvalue (`KismetArrayLibrary.Array_Add` (`self.Colectables`) _colectable))
    (bind (_mesh _id _material) (break `/Game/Colectable` _colectable))
    (bind _new_mesh (`self.CreateStaticMesh` _mesh _material (== _returnvalue 0)))
    (`KismetArrayLibrary.Array_Add` (`self.CollectablesMeshes`) _new_mesh)))

(event `self.DropArea.OnComponentBeginOverlap`
  (params (OverlappedComponent :type "PrimitiveComponent Object Reference") (OtherActor :type "Actor Object Reference") (OtherComp :type "PrimitiveComponent Object Reference") (OtherBodyIndex :type Integer) (bFromSweep :type Boolean) (SweepResult :type "HitResult Structure (by ref)"))
  (bind _asplayer_character (cast `/Game/Blueprints/PlayerCharacter` OtherActor))
  (bind _isplayerone (`/Game/Blueprints/PlayerCharacter.IsPlayerOne` _asplayer_character))
  (if _isplayerone
    (if (== (`self.IsBaseForPlayer1`) true)
      (set `/Game/Blueprints/PlayerCharacter.IsInDropArea` true _asplayer_character :!label _label)
      (set `/Game/Blueprints/PlayerCharacter.HomeBase` self _asplayer_character))
    (elif (== (`self.IsBaseForPlayer1`) false)
      (goto _label))))

(event `self.DropArea.OnComponentEndOverlap`
  (params (OverlappedComponent :type "PrimitiveComponent Object Reference") (OtherActor :type "Actor Object Reference") (OtherComp :type "PrimitiveComponent Object Reference") (OtherBodyIndex :type Integer))
  (bind _asplayer_character (cast `/Game/Blueprints/PlayerCharacter` OtherActor))
  (set `/Game/Blueprints/PlayerCharacter.IsInDropArea` false _asplayer_character))

(fn `CreateStaticMesh`
  (params (Mesh :type "StaticMesh Object Reference") (Material :type "Material Object Reference") (IsFirst :type Boolean))
  (returns (`New Mesh` :type "/Game/Blueprints/CollectableListElement Object Reference"))
  (bind (_returnvalue_x _returnvalue_y _returnvalue_z) (`KismetMathLibrary.BreakVector` (`SceneComponent.K2_GetComponentLocation` (`self.Base`))))
  (bind (_returnvalue_x_2 _returnvalue_y_2 _returnvalue_z_2) (`KismetMathLibrary.BreakVector` (`SceneComponent.K2_GetComponentLocation` (`self.Base`))))
  (if IsFirst
    (bind _returnvalue (`|SpawnActorFromClass` "/Game/Blueprints/CollectableListElement.CollectableListElement_C" (`KismetMathLibrary.MakeTransform` (`KismetMathLibrary.MakeVector` (+ (* (`KismetArrayLibrary.Array_Length` (`self.CollectablesMeshes`)) (`KismetMathLibrary.Conv_IntToDouble` (`self.Offset`))) (- _returnvalue_x 150.0)) _returnvalue_y (+ _returnvalue_z 40.0)) (struct) (0.3 0.3 0.3)) "Undefined" "OverrideRootScale" null null))
    (bind _staticmesh (`/Game/Blueprints/CollectableListElement.StaticMesh` _returnvalue))
    (`StaticMeshComponent.SetStaticMesh` _staticmesh Mesh)
    (`PrimitiveComponent.SetMaterial` _staticmesh 0 Material)
    (return _returnvalue)
    (else
      (bind _returnvalue_2 (`|SpawnActorFromClass` "/Game/Blueprints/CollectableListElement.CollectableListElement_C" (`KismetMathLibrary.MakeTransform` (`KismetMathLibrary.MakeVector` (+ (* (`KismetArrayLibrary.Array_Length` (`self.CollectablesMeshes`)) (`KismetMathLibrary.Conv_IntToDouble` (`self.Offset`))) (- _returnvalue_x_2 150.0)) _returnvalue_y_2 (+ _returnvalue_z_2 40.0)) (struct) (0.3 0.3 0.3)) "Undefined" "OverrideRootScale" null null))
      (bind _staticmesh_2 (`/Game/Blueprints/CollectableListElement.StaticMesh` _returnvalue_2))
      (`StaticMeshComponent.SetStaticMesh` _staticmesh_2 Mesh)
      (`PrimitiveComponent.SetMaterial` _staticmesh_2 0 Material)
      (return _returnvalue_2))))

(fn `DestroyElement`
  (bind _collectablesmeshes (`self.CollectablesMeshes`))
  (bind _outactors (`GameplayStatics.GetAllActorsOfClass` "/Game/Blueprints/CollectableListElement.CollectableListElement_C"))
  (for _array_element _outactors
    (if (`KismetStringLibrary.EqualEqual_StrStr` (`/Game/Blueprints/CollectableListElement.ID` _array_element) (`/Game/Blueprints/CollectableListElement.ID` (`|GetArrayItem` (`self.CollectablesMeshes`))))
      (set `self.ScheduleToDelete` _array_element)
      (set `self.ShouldDeleteMesh` true)))
  ;[1 1 1] Delete only if first mesh was found
  (if (`self.ShouldDeleteMesh`)
    (`GameplayStatics.SpawnEmitterAtLocation` "/Game/Particles/ItemScore_P.ItemScore_P" (`SceneComponent.K2_GetComponentLocation` (`/Game/Blueprints/CollectableListElement.DefaultSceneRoot` (`|GetArrayItem` _collectablesmeshes))))
    (`KismetArrayLibrary.Array_Remove` _collectablesmeshes)
    (`self.K2_DestroyActor` (`self.ScheduleToDelete`))))

(fn `SendVIctoryMessage`
  (bind _outactors (`GameplayStatics.GetAllActorsOfClass` "/Game/Blueprints/PlayerCharacter.PlayerCharacter_C"))
  (for _array_element _outactors
    (bind _isplayerone (`/Game/Blueprints/PlayerCharacter.IsPlayerOne` _array_element))
    (set `/Game/Blueprints/PlayerCharacter.CanMove` false _array_element)
    (if (== (`self.IsBaseForPlayer1`) _isplayerone)
      (bind (_returnvalue_x _returnvalue_y _returnvalue_z) (`KismetMathLibrary.BreakVector` (`SceneComponent.K2_GetComponentLocation` (`Character.Mesh` _array_element))))
      (bind _returnvalue (+ _returnvalue_z 30.0))
      (`GameplayStatics.SpawnEmitterAtLocation` "/Game/Particles/Confetti_P.Confetti_P" (`KismetMathLibrary.MakeVector` _returnvalue_x _returnvalue_y _returnvalue))
      (else
        (`GameplayStatics.SpawnEmitterAtLocation` "/Game/Particles/LoseLightning_P.LoseLightning_P" (`KismetMathLibrary.MakeVector` _returnvalue_x _returnvalue_y _returnvalue))))))

(fn `TryObjectDrop`
  (params (Collectable :type "/Game/Colectable Structure") (`isPlayer 1` :type Boolean))
  (returns (WasDropped :type Boolean))
  (if `isPlayer 1`
    (if (== (`self.IsBaseForPlayer1`) true)
      ;[0 0 0] Is player dropping the right object?
      (if (`KismetStringLibrary.EqualEqual_StrStr` (`.ID_10_51A4873349332FAC86F739BC94859566` (break `/Game/Colectable` Collectable)) (`.ID_10_51A4873349332FAC86F739BC94859566` (break `/Game/Colectable` (`|GetArrayItem` (`self.Colectables`))))) :!label _label
        (`KismetArrayLibrary.Array_Remove` (`self.Colectables`))
        (`self.DestroyElement`)
        ;[0 0 0] CHECK IF IT WAS THE LAST ONE
        (if (== (`KismetArrayLibrary.Array_Length` (`self.CollectablesMeshes`)) 0)
          (`self.SendVIctoryMessage`)
          (`GameplayStatics.PlaySoundAtLocation` (`self.RightObject_SOUND`) (`SceneComponent.K2_GetComponentLocation` (`self.Base`)) (struct) 1.0 1.0 0.0 null null null)
          (return true))
        (else
          (`GameplayStatics.PlaySoundAtLocation` (`self.WrongObject_SOUND`) (`SceneComponent.K2_GetComponentLocation` (`self.Base`)) (struct) 1.0 1.0 0.0 null null null)
          (return false))))
    (elif (== (`self.IsBaseForPlayer1`) false)
      (goto _label))))

(fn `UserConstructionScript`)