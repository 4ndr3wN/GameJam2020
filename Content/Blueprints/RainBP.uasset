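; RainBP is an actor for a falling rain object that moves and spins a static mesh until it hits something.
; Tick applies per-second velocity and rotation to the mesh, without sweep or physics forces.
; On Hit it either destroys itself or, if HoldOnFloor is set, stops moving and counts down HoldOnFloorTimer before destroying itself.
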(event `self.ReceiveTick`
  (params (DeltaSeconds :type "Float (single-precision)"))
  (bind _staticmesh (`self.StaticMesh`))
  (if (`self.IsOnFloor`)
    (bind _output_get (set `self.HoldOnFloorTimer` (- (`self.HoldOnFloorTimer`) DeltaSeconds)))
    (if (<= _output_get 0.0)
      (`self.K2_DestroyActor`))
    (else
      (`SceneComponent.K2_SetWorldLocation` _staticmesh (+ (`SceneComponent.K2_GetComponentLocation` _staticmesh) (* (`self.VelocitySecond`) DeltaSeconds)) false false)
      (`SceneComponent.K2_AddWorldRotation` (`self.StaticMesh`) (* (`self.RotationSecond`) DeltaSeconds) false false))))

(event `self.ReceiveHit`
  (params (MyComp :type "PrimitiveComponent Object Reference") (Other :type "Actor Object Reference") (OtherComp :type "PrimitiveComponent Object Reference") (bSelfMoved :type Boolean) (HitLocation :type "Vector Structure") (HitNormal :type "Vector Structure") (NormalImpulse :type "Vector Structure") (Hit :type "HitResult Structure (by ref)"))
  (if (`self.HoldOnFloor`)
    (set `self.IsOnFloor` true)
    (else
      (`self.K2_DestroyActor`))))

(fn `UserConstructionScript`)