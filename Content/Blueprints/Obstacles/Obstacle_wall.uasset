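; Obstacle wall that alternates between an up and a down position on separate timers, or stays in its starting position when Permanent.
; Tick counts down and flips IsUp, snapping the collision Box to the new marker while the Wall mesh eases after it with delta-scaled interpolation.
; Both timer and movement freeze while a PlayerCharacter overlaps the actor.
; BeginPlay snaps Box and Wall to the initial state.
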(event `self.ReceiveBeginPlay`
  (if (`self.IsUp`)
    (set `self.TimeLeft` (`self.TimeUp`))
    (else
      (set `self.TimeLeft` (`self.TimeDown`))))
  (`self.SetColissionBoxPos` true))

(event `self.ReceiveTick`
  (params (DeltaSeconds :type "Float (single-precision)"))
  (bind _wall (`self.Wall`))
  (bind _returnvalue (`SceneComponent.K2_GetComponentLocation` (`self.Wall`)))
  (bind _returnvalue_2 (`SceneComponent.K2_GetComponentLocation` _wall))
  (if (`self.Permanent`)
    _
    (elif (not (`self.IsOnWall`))
      (`|ExecutionSequence`
        (:`then_0`
          ;[1 1 1] Handle toggling
          (bind _output_get (set `self.TimeLeft` (- (`self.TimeLeft`) DeltaSeconds)))
          (if (< _output_get 0.0)
            (bind _output_get_2 (set `self.IsUp` (not (`self.IsUp`))))
            (if _output_get_2
              (set `self.TimeLeft` (`self.TimeUp`))
              (else
                (set `self.TimeLeft` (`self.TimeDown`))))
            (`self.SetColissionBoxPos` false)))
        (:`then_1`
          (if (`self.IsUp`)
            ;[1 1 1] Move up
            (`SceneComponent.K2_SetWorldLocation` _wall (+ (* (- (`SceneComponent.K2_GetComponentLocation` (`self.UpPosIdentifier`)) _returnvalue_2) DeltaSeconds) _returnvalue_2) false false)
            (else
              ;[1 1 1] Move down
              (`SceneComponent.K2_SetWorldLocation` (`self.Wall`) (+ (* (- (`SceneComponent.K2_GetComponentLocation` (`self.DownPosIdentifier`)) _returnvalue) DeltaSeconds) _returnvalue) false false))))))))

(event `self.ReceiveActorBeginOverlap`
  (params (OtherActor :type "Actor Object Reference"))
  (cast `/Game/Blueprints/PlayerCharacter` OtherActor)
  (set `self.IsOnWall` true))

(event `self.ReceiveActorEndOverlap`
  (params (OtherActor :type "Actor Object Reference"))
  (cast `/Game/Blueprints/PlayerCharacter` OtherActor)
  (set `self.IsOnWall` false))

(fn `SetColissionBoxPos`
  (params (SetWallPos :type Boolean))
  (bind _box (`self.Box`))
  (bind _returnvalue (`SceneComponent.K2_GetComponentLocation` (`self.DownPosIdentifier`)))
  (bind _returnvalue_2 (`SceneComponent.K2_GetComponentLocation` (`self.UpPosIdentifier`)))
  (if (`self.IsUp`)
    (`SceneComponent.K2_SetWorldLocation` _box _returnvalue_2 false false)
    (if SetWallPos
      (`SceneComponent.K2_SetWorldLocation` (`self.Wall`) _returnvalue_2 false false))
    (else
      (`SceneComponent.K2_SetWorldLocation` _box _returnvalue false false)
      (if SetWallPos
        (`SceneComponent.K2_SetWorldLocation` (`self.Wall`) _returnvalue false false)))))

(fn `UserConstructionScript`)