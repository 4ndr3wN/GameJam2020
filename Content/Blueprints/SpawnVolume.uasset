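; Spawn volume actor that scatters collectables and perks at random points and rotations inside its box.
; On BeginPlay it spawns a starting batch of collectables, with types drawn from the CustomGameInstance.
; Tick counts down a randomized delay, then rolls against PercentageOfCollectable to spawn either another collectable or one of four random perk classes.
; Both spawn functions call themselves again if the spawned actor is invalid.
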(event `self.ReceiveBeginPlay`
  (`self.ResetTimeToNextAction`)
  (bind _ascustom_game_instance (cast `/Game/CustomGameInstance` (`GameplayStatics.GetGameInstance`)))
  (bind _output_get (set `self.GameInstance_REF` _ascustom_game_instance))
  (for _ (range (`self.StartingColectables`))
    (bind _colectable (`/Game/CustomGameInstance.GetRandomCollectable` _output_get))
    (`self.SpawnColectable` _colectable)))

(event `self.ReceiveTick`
  (params (DeltaSeconds :type "Float (single-precision)"))
  (bind _output_get (set `self.TimeToNextAction` (- (`self.TimeToNextAction`) DeltaSeconds)))
  (if (< _output_get 0.0)
    (`self.ResetTimeToNextAction`)
    (if (<= (`KismetMathLibrary.RandomIntegerInRange` 0 100) (`self.PercentageOfCollectable`))
      (bind _colectable (`/Game/CustomGameInstance.GetRandomCollectable` (`self.GameInstance_REF`)))
      (`self.SpawnColectable` _colectable)
      (else
        (`self.SpawnPerk`)))))

(fn `ResetTimeToNextAction`
  (set `self.TimeToNextAction` (`KismetMathLibrary.RandomFloatInRange` 6.0 11.0)))

(fn `SpawnColectable`
  (params (`Actor Type` :type "/Game/Colectable Structure"))
  (bind _volume (`self.Volume`))
  (bind _returnvalue (`|SpawnActorFromClass` "/Game/Blueprints/Collectable.Collectable_C" (`KismetMathLibrary.MakeTransform` (`KismetMathLibrary.RandomPointInBoundingBox` (`SceneComponent.K2_GetComponentLocation` _volume) (`BoxComponent.GetScaledBoxExtent` _volume)) (`KismetMathLibrary.RandomRotator` false)) "AdjustIfPossibleButAlwaysSpawn" "OverrideRootScale" null `Actor Type` null))
  (`/Engine/EditorBlueprintResources/StandardMacros.IsValid` _returnvalue
    (:`Is Valid`
      (`KismetSystemLibrary.PrintString` "Collectable!"))
    (:`Is Not Valid`
      (`self.SpawnColectable` `Actor Type`))))

(fn `SpawnPerk`
  (bind _volume (`self.Volume`))
  (bind _volume_2 (`self.Volume`))
  (bind _volume_3 (`self.Volume`))
  (bind _volume_4 (`self.Volume`))
  (switch `int` (`KismetMathLibrary.RandomIntegerInRange` 0 3)
    (:`0`
      (bind _returnvalue (`|SpawnActorFromClass` "/Game/Blueprints/Perks/Perk1.Perk1_C" (`KismetMathLibrary.MakeTransform` (`KismetMathLibrary.RandomPointInBoundingBox` (`SceneComponent.K2_GetComponentLocation` _volume_3) (`BoxComponent.GetScaledBoxExtent` _volume_3)) (`KismetMathLibrary.RandomRotator` false)) "AdjustIfPossibleButAlwaysSpawn" "OverrideRootScale" null null))
      (`/Engine/EditorBlueprintResources/StandardMacros.IsValid` _returnvalue
        (:`Is Not Valid`
          (`self.SpawnPerk`))))
    (:`1`
      (bind _returnvalue_2 (`|SpawnActorFromClass` "/Game/Blueprints/Perks/Perk2.Perk2_C" (`KismetMathLibrary.MakeTransform` (`KismetMathLibrary.RandomPointInBoundingBox` (`SceneComponent.K2_GetComponentLocation` _volume_4) (`BoxComponent.GetScaledBoxExtent` _volume_4)) (`KismetMathLibrary.RandomRotator` false)) "AdjustIfPossibleButAlwaysSpawn" "OverrideRootScale" null null))
      (`/Engine/EditorBlueprintResources/StandardMacros.IsValid` _returnvalue_2
        (:`Is Not Valid`
          (`self.SpawnPerk`))))
    (:`2`
      (bind _returnvalue_3 (`|SpawnActorFromClass` "/Game/Blueprints/Perks/Perk3.Perk3_C" (`KismetMathLibrary.MakeTransform` (`KismetMathLibrary.RandomPointInBoundingBox` (`SceneComponent.K2_GetComponentLocation` _volume_2) (`BoxComponent.GetScaledBoxExtent` _volume_2)) (`KismetMathLibrary.RandomRotator` false)) "AdjustIfPossibleButAlwaysSpawn" "OverrideRootScale" null null))
      (`/Engine/EditorBlueprintResources/StandardMacros.IsValid` _returnvalue_3
        (:`Is Not Valid`
          (`self.SpawnPerk`))))
    (:`3`
      (bind _returnvalue_4 (`|SpawnActorFromClass` "/Game/Blueprints/Perks/Perk4.Perk4_C" (`KismetMathLibrary.MakeTransform` (`KismetMathLibrary.RandomPointInBoundingBox` (`SceneComponent.K2_GetComponentLocation` _volume) (`BoxComponent.GetScaledBoxExtent` _volume)) (`KismetMathLibrary.RandomRotator` false)) "AdjustIfPossibleButAlwaysSpawn" "OverrideRootScale" null null))
      (`/Engine/EditorBlueprintResources/StandardMacros.IsValid` _returnvalue_4
        (:`Is Not Valid`
          (`self.SpawnPerk`))))))

(fn `UserConstructionScript`)